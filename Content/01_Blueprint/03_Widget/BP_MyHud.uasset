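; BP_MyHud is a HUD Blueprint that manages the game's main UI and a toggleable settings screen.
; On BeginPlay it creates WBP_MainUI for the first player controller, shows it in the viewport, and calls its SetTime every Tick.
; ShowSettingUI lazily creates WBP_SettingUI on first use, then flips it between Visible and Collapsed using the IsSettingVisible flag.
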(event `Show Setting UI`
  (bind _settingui (`self.SettingUI`))
  (`/Engine/EditorBlueprintResources/StandardMacros.IsValid` (`self.SettingUI`)
    (:`Is Valid`
      _)
    (:`Is Not Valid`
      (bind _returnvalue (`|CreateWidget` "/Game/01_Blueprint/03_Widget/WBP_SettingUI.WBP_SettingUI_C" (`self.PlayerController`)))
      (bind _output_get (set `self.SettingUI` _returnvalue))
      (`UserWidget.AddToViewport` _output_get 0)))
  (if (`self.IsSettingVisible`)
    (`Widget.SetVisibility` _settingui "Collapsed")
    (else
      (`Widget.SetVisibility` _settingui "Visible")))
  (set `self.IsSettingVisible` (not (`self.IsSettingVisible`))))

(event `self.ReceiveBeginPlay`
  (bind _output_get (set `self.PlayerController` (`GameplayStatics.GetPlayerController` 0)))
  (bind _returnvalue (`|CreateWidget` "/Game/01_Blueprint/03_Widget/WBP_MainUI.WBP_MainUI_C" _output_get))
  (bind _output_get_2 (set `self.MainUI` _returnvalue))
  (`UserWidget.AddToViewport` _output_get_2 0)
  (set `Widget.Visibility` "Visible" _output_get_2))

(event `self.ReceiveTick`
  (params (DeltaSeconds :type "Float (single-precision)"))
  (`/Game/01_Blueprint/03_Widget/WBP_MainUI.SetTime` (`self.MainUI`)))

(fn `UserConstructionScript`)