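; BP_UpgradedCube is an actor that moves back and forth along the direction of its Arrow component's relative location.
; Tick offsets the position by Speed, delta time and Direction without sweeping, applying that relative vector directly in world space.
; Direction flips once the actor is at least 50 units from its start, with a half-second timer preventing immediate re-flips.
; The target direction computed at BeginPlay and a timer-only reversal branch are unused.
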(event `self.ReceiveBeginPlay`
  (bind _output_get (set `self.StartPos` (`self.K2_GetActorLocation`)))
  (bind _output_get_2 (set `self.Pos` _output_get))
  (bind _output_get_3 (set `self.TargetPos` (- (`SceneComponent.K2_GetComponentLocation` (`self.Arrow`)) _output_get_2)))
  (set `self.TargetDir` (`KismetMathLibrary.Normal` _output_get_3)))

(event `self.ReceiveTick`
  (params (DeltaSeconds :type "Float (single-precision)"))
  (bind _returnvalue (+ (* (`KismetMathLibrary.Normal` (`SceneComponent.RelativeLocation` (`self.Arrow`))) (* (`self.RealSpeed`) (`self.Direction`))) (`self.Pos`)))
  (set `self.RealSpeed` (* DeltaSeconds (`self.Speed`)))
  (set `self.timer` (+ DeltaSeconds (`self.timer`)))
  (`self.K2_SetActorLocation` _returnvalue)
  (set `self.Pos` _returnvalue)
  (if (>= (`KismetMathLibrary.VSize` (- (`self.K2_GetActorLocation`) (`self.StartPos`))) 50.0)
    (if (> (`self.timer`) 0.5)
      (set `self.Direction` (* (`self.Direction`) -1.0))
      (set `self.timer` 0.0))))

(fn `UserConstructionScript`)