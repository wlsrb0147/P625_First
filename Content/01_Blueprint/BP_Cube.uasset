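; BP_Cube is an actor that moves back and forth along a configurable axis.
; Each Tick advances its stored position along MoveDir, scaled by Speed, Direction and delta time, then sets the actor location without sweeping.
; An accumulated timer reverses Direction and resets once it exceeds three seconds.
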(event `self.ReceiveBeginPlay`)

(event `self.ReceiveTick`
  (params (DeltaSeconds :type "Float (single-precision)"))
  (set `self.RealSpeed` (* DeltaSeconds (`self.Speed`)))
  (set `self.timer` (+ DeltaSeconds (`self.timer`)))
  (bind _output_get (set `self.Pos` (+ (* (`self.RealSpeed`) (`self.Direction`) (`self.MoveDir`)) (`self.Pos`))))
  (`self.K2_SetActorLocation` _output_get)
  (if (> (`self.timer`) 3.0)
    (set `self.Direction` (* (`self.Direction`) -1.0))
    (set `self.timer` 0.0)))

(fn `UserConstructionScript`)