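; BP_Projectile is a physics-driven projectile that sets off a field system actor where it hits.
; On BeginPlay it launches its static mesh along the actor's forward vector with a single large mass-independent force.
; On Hit it spawns an FS_MasterField at the impact location, sets its activation type and triggers it, then destroys itself after a short delay.
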(event `self.ReceiveBeginPlay`
  (`PrimitiveComponent.AddForce` (`self.StaticMesh`) (* (`self.GetActorForwardVector` self) 1000000.0) "None" true))

(event `self.ReceiveHit`
  (params (MyComp :type "PrimitiveComponent Object Reference") (Other :type "Actor Object Reference") (OtherComp :type "PrimitiveComponent Object Reference") (bSelfMoved :type Boolean) (HitLocation :type "Vector Structure") (HitNormal :type "Vector Structure") (NormalImpulse :type "Vector Structure") (Hit :type "HitResult Structure (by ref)"))
  (bind _returnvalue (`|SpawnActorFromClass` "/Engine/EditorResources/FieldNodes/FS_MasterField.FS_MasterField_C" (`KismetMathLibrary.MakeTransform` HitLocation) "Undefined" "MultiplyWithRoot" null null))
  (set `/Engine/EditorResources/FieldNodes/FS_MasterField.ActivationType` "NewEnumerator4" _returnvalue)
  (`/Engine/EditorResources/FieldNodes/FS_MasterField.CE_Trigger` _returnvalue)
  (`KismetSystemLibrary.Delay` 0.2)
  (`self.K2_DestroyActor`))

(fn `UserConstructionScript`)