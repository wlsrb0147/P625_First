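; BP_MonsterProjectile is a monster projectile that knocks the player character back on contact, with no damage logic in this Blueprint.
; On BeginPlay it propels its static mesh along the actor's forward vector with a single physics force applied as an acceleration change.
; When its sphere overlaps a BP_Character, it adds a small launch velocity pointing away from the projectile, then destroys itself.
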(event `self.ReceiveBeginPlay`
  (`PrimitiveComponent.AddForce` (`self.StaticMesh`) (* (`self.GetActorForwardVector` self) 1000000.0) "None" true))

(event `self.Sphere.OnComponentBeginOverlap`
  (params (OverlappedComponent :type "PrimitiveComponent Object Reference") (OtherActor :type "Actor Object Reference") (OtherComp :type "PrimitiveComponent Object Reference") (OtherBodyIndex :type Integer) (bFromSweep :type Boolean) (SweepResult :type "HitResult Structure (by ref)"))
  (bind _asbp_character (cast `/Game/01_Blueprint/01_Character/BP_Character` OtherActor))
  (`/Engine/EditorBlueprintResources/StandardMacros.IsValid` null
    (:`Is Valid`
      (`Character.LaunchCharacter` _asbp_character (* (`KismetMathLibrary.Normal` (- (`self.K2_GetActorLocation` _asbp_character) (`self.K2_GetActorLocation`) (0.0 0.0 0.0))) 100.0) false false)
      (`self.K2_DestroyActor`))))

(fn `UserConstructionScript`)