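; BP_InteractionActor is an interaction actor that shows a timed progress indicator through its widget.
; BeginPlay gets a dynamic material from an image in WBP_whatisit.
; While IsInteracting is true, Tick counts down the remaining time and writes its ratio to the material's Percent parameter.
; Two DoOnce gates re-arm each other, so the timer and indicator reset once when interaction stops.
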(event `self.ReceiveBeginPlay`
  (bind _aswbp_whatisit (cast `/Game/01_Blueprint/03_Widget/WBP_whatisit` (`WidgetComponent.GetWidget` (`self.Widget`))))
  (bind _returnvalue (`Image.GetDynamicMaterial` (`/Game/01_Blueprint/03_Widget/WBP_whatisit.Image_26` _aswbp_whatisit)))
  (set `self.Dynamic` _returnvalue))

(event `self.ReceiveTick`
  (params (DeltaSeconds :type "Float (single-precision)"))
  (if (`self.IsInteracting`)
    (if (> (`self.InteractingTimeLeft`) 0.0)
      (bind _output_get (set `self.InteractingTimeLeft` (- (`self.InteractingTimeLeft`) DeltaSeconds)))
      (bind _output_get_2 (set `self.Percentage` (/ _output_get (`self.InitialInteractingTime`))))
      (`MaterialInstanceDynamic.SetScalarParameterValue` (`self.Dynamic`) "Percent" _output_get_2)
      (`/Engine/EditorBlueprintResources/StandardMacros.DoOnce` false :!label _label
        (:`Completed`
          (goto _label_2 :!via `Reset`))))
    (else
      (`/Engine/EditorBlueprintResources/StandardMacros.DoOnce` false :!label _label_2
        (:`Completed`
          (set `self.InteractingTimeLeft` 3.0)
          (bind _output_get_3 (set `self.Percentage` 1.0))
          (`MaterialInstanceDynamic.SetScalarParameterValue` (`self.Dynamic`) "Percent" _output_get_3)
          (goto _label :!via `Reset`))))))

(fn `UserConstructionScript`)