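; BP_TMyCharacter is a test player character with basic movement, jump and mouse look through Enhanced Input.
; On BeginPlay it casts its controller to PlayerController and adds the IA_TController mapping context, printing a message if the cast fails.
; Forward and right input move it along directions derived from control yaw only, so camera pitch does not affect movement.
; Mouse input drives controller yaw and pitch.
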(event `self.ReceiveBeginPlay`
  (bind `_as플레이어_컨트롤러` (cast `PlayerController` (`self.GetController`))
    (:`then`
      (`/Engine/EditorBlueprintResources/StandardMacros.IsValid` `_as플레이어_컨트롤러`
        (:`Is Valid`
          (`EnhancedInputSubsystemInterface.AddMappingContext` (pcsubsystem `EnhancedInputLocalPlayerSubsystem` `_as플레이어_컨트롤러`) "/Game/01_Blueprint/99_MyTest/IA_TController.IA_TController" 0 (struct)))))
    (:`CastFailed`
      (`KismetSystemLibrary.PrintString` "캐스팅 실패"))))

(event `EnhancedInput|/Game/01_Blueprint/99_MyTest/IA_TForward`
  (params (ActionValue :type "Float (double-precision)") (ElapsedSeconds :type "Float (double-precision)") (TriggeredSeconds :type "Float (double-precision)") (InputAction :type "InputAction Object Reference" :default "/Game/01_Blueprint/99_MyTest/IA_TForward.IA_TForward"))
  (bind (_returnvalue_roll _returnvalue_pitch _returnvalue_yaw) (`KismetMathLibrary.BreakRotator` (`self.GetControlRotation`)))
  (:`Triggered`
    (`self.AddMovementInput` (`KismetMathLibrary.GetForwardVector` (`KismetMathLibrary.MakeRotator` 0.0 0.0 _returnvalue_yaw)) ActionValue)))

(event `EnhancedInput|/Game/01_Blueprint/99_MyTest/IA_TRight`
  (params (ActionValue :type "Float (double-precision)") (ElapsedSeconds :type "Float (double-precision)") (TriggeredSeconds :type "Float (double-precision)") (InputAction :type "InputAction Object Reference" :default "/Game/01_Blueprint/99_MyTest/IA_TRight.IA_TRight"))
  (bind (_returnvalue_roll _returnvalue_pitch _returnvalue_yaw) (`KismetMathLibrary.BreakRotator` (`self.GetControlRotation`)))
  (:`Triggered`
    (`self.AddMovementInput` (`KismetMathLibrary.GetRightVector` (`KismetMathLibrary.MakeRotator` 0.0 0.0 _returnvalue_yaw)) ActionValue)))

(event `EnhancedInput|/Game/01_Blueprint/99_MyTest/IA_TJump`
  (params (ActionValue :type Boolean) (ElapsedSeconds :type "Float (double-precision)") (TriggeredSeconds :type "Float (double-precision)") (InputAction :type "InputAction Object Reference" :default "/Game/01_Blueprint/99_MyTest/IA_TJump.IA_TJump"))
  (:`Started`
    (`self.Jump`)))

(event `EnhancedInput|/Game/01_Blueprint/99_MyTest/IA_TMouse`
  (params (ActionValue :type "Vector2D Structure") (ElapsedSeconds :type "Float (double-precision)") (TriggeredSeconds :type "Float (double-precision)") (InputAction :type "InputAction Object Reference" :default "/Game/01_Blueprint/99_MyTest/IA_TMouse.IA_TMouse"))
  (:`Triggered`
    (`self.AddControllerYawInput` ActionValue_X)
    (`self.AddControllerPitchInput` ActionValue_Y)))

(fn `UserConstructionScript`)