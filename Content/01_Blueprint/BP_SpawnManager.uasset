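; BP_SpawnManager is a timed monster spawner configured through SpawnFromData.
; SpawnFromData stores monster rows, interval, count and radius, then starts a looping timer once via DoOnce.
; Each tick of that timer looks up a random data table row and spawns its actor class.
; Count and radius go unused: spawns never stop here and land at a random unit vector, unrelated to the manager's position.
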(event `SpawnFromData`
  (params (Count :type "/Game/03_DataDable/Str_SpawnData Structure"))
  (set `self.Count Monster Data` Count_MonsterData_8_9F4CB2ED4587F4403A36718DA3775037)
  (set `self.Count Spawn Time_0` Count_SpawnTime_14_33A5C33842B1FB69DD8633B5FBBF1787)
  (set `self.Count Spawn Count_0` Count_SpawnCount_15_182868474D0B143BF588E886DE3E4464)
  (set `self.Count Radius` Count_Radius_18_338C564E45CABBE3AC0B24AA433A63FB)
  (`/Engine/EditorBlueprintResources/StandardMacros.DoOnce` false
    (:`Completed`
      (`self.SpawnStart` (struct)))))

(event `SpawnStart`
  (params (NewParam :type "/Game/03_DataDable/Str_SpawnData Structure"))
  (bind _returnvalue (`KismetSystemLibrary.K2_SetTimerDelegate` (delegate `Spawn`) (`self.Count Spawn Time_0`) true))
  (set `self.Timer` _returnvalue))

(event `Spawn`
  (bind (_datatable _rowname) (break `DataTableRowHandle` (`KismetArrayLibrary.Array_Random` (`self.Count Monster Data`))))
  (bind _returnvalue (`|GetDataTableRow` _datatable _rowname)
    (:`then`
      (`|SpawnActorFromClass` (`.MemberVar_1_2_0C9C6BA7408D6CB3DA04E2940A9B0361` (break `/Game/03_DataDable/Str_MonsterData` _returnvalue)) (`KismetMathLibrary.MakeTransform` (`KismetMathLibrary.RandomUnitVectorInConeInDegrees` (0.0 0.0 0.0) 150.0)) "Undefined" "MultiplyWithRoot" null null))))

(fn `UserConstructionScript`)