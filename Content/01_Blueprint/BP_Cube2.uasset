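; BP_Cube2 is a cube actor that offers an interaction to the player character while it is within range.
; When a BP_Character enters its InteractionSphere, it spawns a BP_InteractionActor at its own location and assigns the reference to the character.
; When the character leaves, it destroys that spawned actor without explicitly clearing the character's reference.
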(event `self.InteractionSphere.OnComponentBeginOverlap`
  (params (OverlappedComponent :type "PrimitiveComponent Object Reference") (OtherActor :type "Actor Object Reference") (OtherComp :type "PrimitiveComponent Object Reference") (OtherBodyIndex :type Integer) (bFromSweep :type Boolean) (SweepResult :type "HitResult Structure (by ref)"))
  (bind _asbp_character (cast `/Game/01_Blueprint/01_Character/BP_Character` OtherActor))
  (set `self.Player` _asbp_character)
  (bind _returnvalue (`|SpawnActorFromClass` "/Game/01_Blueprint/BP_InteractionActor.BP_InteractionActor_C" (`KismetMathLibrary.MakeTransform` (`self.K2_GetActorLocation`)) "Undefined" "MultiplyWithRoot" null null))
  (bind _output_get (set `self.InteractionActor` _returnvalue))
  (set `/Game/01_Blueprint/01_Character/BP_Character.InteractionActor` _output_get (`self.Player`)))

(event `self.InteractionSphere.OnComponentEndOverlap`
  (params (OverlappedComponent :type "PrimitiveComponent Object Reference") (OtherActor :type "Actor Object Reference") (OtherComp :type "PrimitiveComponent Object Reference") (OtherBodyIndex :type Integer))
  (cast `/Game/01_Blueprint/01_Character/BP_Character` OtherActor)
  (`self.K2_DestroyActor` (`self.InteractionActor`)))

(fn `UserConstructionScript`)