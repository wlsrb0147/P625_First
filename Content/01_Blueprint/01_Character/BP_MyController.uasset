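; BP_MyController is a player controller that sets up Enhanced Input and opens the settings UI on the inventory input action.
; On BeginPlay it adds the ControllerInput mapping context, caches BP_MyHud and hides the mouse cursor.
; IAU_OpenInven calls the HUD's ShowSettingUI, then uses the CursorVisible flag to alternate between GameAndUI and GameOnly input modes.
; The toggle flips and prints that flag but never updates ShowMouseCursor.
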(event `self.ReceiveBeginPlay`
  (`EnhancedInputSubsystemInterface.AddMappingContext` (pcsubsystem `EnhancedInputLocalPlayerSubsystem` self) "/Game/01_Blueprint/00_Global/00_Input/ControllerInput.ControllerInput" 0 (struct))
  (bind _asbp_my_hud (cast `/Game/01_Blueprint/03_Widget/BP_MyHud` (`self.GetHUD`)))
  (set `self.Hud` _asbp_my_hud)
  (bind _output_get (set `self.bShowMouseCursor` false))
  (set `self.CursorVisible` _output_get))

(event `EnhancedInput|/Game/01_Blueprint/00_Global/00_Input/IAU_OpenInven`
  (params (ActionValue :type Boolean) (ElapsedSeconds :type "Float (double-precision)") (TriggeredSeconds :type "Float (double-precision)") (InputAction :type "InputAction Object Reference" :default "/Game/01_Blueprint/00_Global/00_Input/IAU_OpenInven.IAU_OpenInven"))
  (:`Started`
    (`/Game/01_Blueprint/03_Widget/BP_MyHud.Show Setting UI` (`self.Hud`))
    (if (`self.CursorVisible`)
      (`WidgetBlueprintLibrary.SetInputMode_GameOnly` self)
      (else
        (`WidgetBlueprintLibrary.SetInputMode_GameAndUIEx` self null)))
    (bind _output_get (set `self.CursorVisible` (not (`self.CursorVisible`))))
    (`KismetSystemLibrary.PrintString` (`KismetStringLibrary.Conv_BoolToString` _output_get))))

(fn `UserConstructionScript`)