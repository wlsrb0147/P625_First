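; Player character Blueprint with Enhanced Input movement, projectile firing, montage combo attacks and F-key interaction.
; Footstep events trace the ground and use PM_Base physical materials to choose Niagara effects, sounds and decals.
; Attack sphere-traces forward, lowering the character's own HP on the HUD and spawning randomized damage actors on hits.
; Jumping spawns a temporary pose-copied BP_Car, Add sends DigStoneMessage to nearby actors, and a scene capture shows only this character.
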(event `self.ReceiveBeginPlay`
  ;[1 1 1] 비긴 플레이
  (bind `_as플레이어_컨트롤러` (cast `PlayerController` (`self.GetController`)))
  (`/Engine/EditorBlueprintResources/StandardMacros.IsValid` `_as플레이어_컨트롤러`
    (:`Is Valid`
      (`EnhancedInputSubsystemInterface.AddMappingContext` (pcsubsystem `EnhancedInputLocalPlayerSubsystem` `_as플레이어_컨트롤러`) "/Game/01_Blueprint/00_Global/00_Input/CharacterInput.CharacterInput" 0 (struct))
      (set `self.Anim` (`SkeletalMeshComponent.GetAnimInstance` (`self.Mesh`)))
      (bind _asbp_my_hud (cast `/Game/01_Blueprint/03_Widget/BP_MyHud` (`PlayerController.GetHUD` (`GameplayStatics.GetPlayerController` 0))))
      (bind _output_get (set `self.My Hud` _asbp_my_hud))
      (bind _mainui (`/Game/01_Blueprint/03_Widget/BP_MyHud.MainUI` _output_get)
        (:`then`
          (set `self.Main UI` _mainui))
        (:`else`)))))

(event `EnhancedInput|/Game/01_Blueprint/00_Global/00_Input/IA_Jump`
  (params (ActionValue :type Boolean) (ElapsedSeconds :type "Float (double-precision)") (TriggeredSeconds :type "Float (double-precision)") (InputAction :type "InputAction Object Reference" :default "/Game/01_Blueprint/00_Global/00_Input/IA_Jump.IA_Jump"))
  ;[1 1 1] 움직임 조작
  (:`Started`
    (`self.Jump`)
    (bind _returnvalue (`|SpawnActorFromClass` "/Game/01_Blueprint/BP_Car.BP_Car_C" (`SceneComponent.K2_GetComponentToWorld` (`self.Mesh`)) "Undefined" "MultiplyWithRoot" null null))
    (`/Game/01_Blueprint/BP_Car.CopyPose` _returnvalue (`self.Mesh`))
    (`KismetSystemLibrary.Delay` 5.0)
    (`self.K2_DestroyActor` _returnvalue)))

(event `EnhancedInput|/Game/01_Blueprint/00_Global/00_Input/IA_MouseXY`
  (params (ActionValue :type "Vector2D Structure") (ElapsedSeconds :type "Float (double-precision)") (TriggeredSeconds :type "Float (double-precision)") (InputAction :type "InputAction Object Reference" :default "/Game/01_Blueprint/00_Global/00_Input/IA_MouseXY.IA_MouseXY"))
  ;[1 1 1] 움직임 조작
  (:`Triggered`
    (`self.AddControllerYawInput` ActionValue_X)
    (`self.AddControllerPitchInput` ActionValue_Y)))

(event `EnhancedInput|/Game/01_Blueprint/00_Global/00_Input/IA_MoveForward`
  (params (ActionValue :type "Float (double-precision)") (ElapsedSeconds :type "Float (double-precision)") (TriggeredSeconds :type "Float (double-precision)") (InputAction :type "InputAction Object Reference" :default "/Game/01_Blueprint/00_Global/00_Input/IA_MoveForward.IA_MoveForward"))
  (bind (_returnvalue_roll _returnvalue_pitch _returnvalue_yaw) (`KismetMathLibrary.BreakRotator` (`self.GetControlRotation`)))
  ;[1 1 1] 움직임 조작
  (:`Triggered`
    (`self.AddMovementInput` (`KismetMathLibrary.GetForwardVector` (`KismetMathLibrary.MakeRotator` 0.0 0.0 _returnvalue_yaw)) ActionValue)))

(event `EnhancedInput|/Game/01_Blueprint/00_Global/00_Input/IA_Right`
  (params (ActionValue :type "Float (double-precision)") (ElapsedSeconds :type "Float (double-precision)") (TriggeredSeconds :type "Float (double-precision)") (InputAction :type "InputAction Object Reference" :default "/Game/01_Blueprint/00_Global/00_Input/IA_Right.IA_Right"))
  (bind (_returnvalue_roll _returnvalue_pitch _returnvalue_yaw) (`KismetMathLibrary.BreakRotator` (`self.GetControlRotation`)))
  ;[1 1 1] 움직임 조작
  (:`Triggered`
    (`self.AddMovementInput` (`KismetMathLibrary.GetRightVector` (`KismetMathLibrary.MakeRotator` 0.0 0.0 _returnvalue_yaw)) ActionValue)))

(event `EnhancedInput|/Game/01_Blueprint/00_Global/00_Input/IA_Q`
  (params (ActionValue :type Boolean) (ElapsedSeconds :type "Float (double-precision)") (TriggeredSeconds :type "Float (double-precision)") (InputAction :type "InputAction Object Reference" :default "/Game/01_Blueprint/00_Global/00_Input/IA_Q.IA_Q"))
  ;[1 1 1] Q누르면 애니메이션 재생
  (:`Started`
    (`AnimInstance.Montage_Play` (`self.Anim`) "/Game/01_Blueprint/02_Resource/Character/SkeletalMesh/Boris/AMT_Kettle.AMT_Kettle" 1.0 "MontageLength" 0.0 true)))

(event `EnhancedInput|/Game/01_Blueprint/00_Global/00_Input/IA_MouseLeftClick`
  (params (ActionValue :type Boolean) (ElapsedSeconds :type "Float (double-precision)") (TriggeredSeconds :type "Float (double-precision)") (InputAction :type "InputAction Object Reference" :default "/Game/01_Blueprint/00_Global/00_Input/IA_MouseLeftClick.IA_MouseLeftClick"))
  (bind (_returnvalue_location _returnvalue_rotation) (`KismetMathLibrary.BreakTransform` (`self.GetTransform`)))
  ;[1 1 1] 좌클릭시 탄환 발사
  (:`Started`
    (`|SpawnActorFromClass` "/Game/01_Blueprint/BP_Projectile.BP_Projectile_C" (`KismetMathLibrary.MakeTransform` (+ _returnvalue_location (* (`self.GetActorForwardVector`) 2)) _returnvalue_rotation) "Undefined" "MultiplyWithRoot" null null)))

(event `EnhancedInput|/Game/01_Blueprint/00_Global/00_Input/IA_RightClick`
  (params (ActionValue :type Boolean) (ElapsedSeconds :type "Float (double-precision)") (TriggeredSeconds :type "Float (double-precision)") (InputAction :type "InputAction Object Reference" :default "/Game/01_Blueprint/00_Global/00_Input/IA_RightClick.IA_RightClick"))
  ;[1 1 1] 공격 입력
  (:`Started`
    (if (`self.IsAttacking`)
      (if (`self.ComboTiming`)
        (`AnimInstance.Montage_Play` (`self.Anim`) "/Game/01_Blueprint/02_Resource/Character/SkeletalMesh/Boris/ATM_Boris_Atk2.ATM_Boris_Atk2" 1.0 "MontageLength" 0.0 true))
      (else
        (`AnimInstance.Montage_Play` (`self.Anim`) "/Game/01_Blueprint/02_Resource/Character/SkeletalMesh/Boris/AMT_Boris_Atk.AMT_Boris_Atk" 1.0 "MontageLength" 0.0 true)))))

(event `FootStep`
  (params (IsLeft :type Boolean))
  (bind _mesh (`self.Mesh`))
  (bind _footlocation (`self.FootLocation`))
  (bind _location (`self.Location`))
  (bind (_bblockinghit _binitialoverlap _time _distance _location_2 _impactpoint _normal _impactnormal _physmat) (`GameplayStatics.BreakHitResult` (`self.Out Hit`)))
  ;[1 1 1] 걸을때 나이아가라 생성
  (`|ExecutionSequence`
    (:`then_0`
      (if IsLeft
        (set `self.FootLocation` (`SceneComponent.GetSocketLocation` _mesh "Foot_L"))
        (else
          (set `self.FootLocation` (`SceneComponent.GetSocketLocation` _mesh "Foot_R"))))
      (bind (_outhit _returnvalue) (`KismetSystemLibrary.LineTraceSingle` :`Start` _footlocation :`End` (+ _footlocation (0.0 0.0 -150.0)) :`TraceChannel` "TraceTypeQuery3" :`DrawDebugType` "ForDuration" :`DrawTime` 2.0))
      (if _returnvalue
        (set `self.Out Hit` _outhit)))
    (:`then_1`
      (bind _aspm_base (cast `/Game/01_Blueprint/02_Resource/Material/PM_Base` _physmat))
      (bind _output_get (set `self.Location` (+ _impactpoint (0.0 0.0 20.0))))
      (bind _returnvalue_2 (`NiagaraFunctionLibrary.SpawnSystemAtLocation` (`/Game/01_Blueprint/02_Resource/Material/PM_Base.FootWalk` _aspm_base) _output_get (`SceneComponent.K2_GetComponentRotation` (`self.Mesh`)) (1.0 1.0 1.0) true true "AutoRelease"))
      (`GameplayStatics.PlaySoundAtLocation` (`/Game/01_Blueprint/02_Resource/Material/PM_Base.FootSound` _aspm_base) _impactpoint (struct) 1.0 1.0 0.0 null null null null)
      (`KismetSystemLibrary.Delay` 0.5)
      (`ActorComponent.K2_DestroyComponent` _returnvalue_2)
      (if true
        (`|SpawnActorFromClass` (`/Game/01_Blueprint/02_Resource/Material/PM_Base.Decal` _aspm_base) (`KismetMathLibrary.MakeTransform` _location) "Undefined" "MultiplyWithRoot" null null)
        (else
          (`GameplayStatics.SpawnDecalAtLocation` "/Game/01_Blueprint/02_Resource/Material/M_Decal.M_Decal" (100.0 100.0 100.0) _location))))))

(event `Attack`
  (bind _returnvalue (`self.K2_GetActorLocation`))
  (bind _radius (`self.Radius`))
  (bind _returnvalue_2 (+ _returnvalue (* (`self.GetActorForwardVector`) (`self.NewVar_0`))))
  (`|ExecutionSequence` :!label _label
    (:`then_0`
      ;[1 1 1] 공격 실행
      (bind (_outhit _returnvalue_3) (`KismetSystemLibrary.SphereTraceSingleByProfile` _returnvalue _returnvalue_2 _radius "PlayerAttack"))
      (`KismetSystemLibrary.DrawDebugSphere` _returnvalue_2 _radius 12 (struct :`R` 1.0 :`G` 1.0 :`B` 1.0 :`A` 1.0) 2.0)
      (if _returnvalue_3
        (if (> (`self.CurrentHp`) 0.0)
          (bind _output_get (set `self.CurrentHp` (- (`self.CurrentHp`) 0.1)))
          (`/Game/01_Blueprint/03_Widget/WBP_MainUI.SetHp` (`self.Main UI`) _output_get)
          (bind _returnvalue_4 (`|SpawnActorFromClass` "/Game/01_Blueprint/BP_DamageActor.BP_DamageActor_C" (`KismetMathLibrary.MakeTransform` (`.Location` (`GameplayStatics.BreakHitResult` _outhit))) "AlwaysSpawn" "MultiplyWithRoot" null null))
          (`/Game/01_Blueprint/BP_DamageActor.Init_DamageActor` _returnvalue_4 (`KismetMathLibrary.RandomInteger64InRange` 1 100) (`KismetMathLibrary.RandomBool`)))))))

(event `PlayAttack`
  (goto _label))

(event `Key|Add`
  (params (Key :type "Key Structure"))
  (bind _returnvalue (`self.K2_GetActorLocation`))
  (:`Pressed`
    (bind _outhits (`KismetSystemLibrary.SphereTraceMultiByProfile` :`Start` _returnvalue :`End` _returnvalue :`Radius` 500.0 :`ProfileName` "BlockAll" :`DrawDebugType` "ForDuration" :`DrawTime` 3.0))
    (for _array_element _outhits
      (message `/Game/01_Blueprint/04_NPC/BPI_Dig.DigStone` (`.HitActor` (`GameplayStatics.BreakHitResult` _array_element))))))

(event `Key|F`
  (params (Key :type "Key Structure"))
  (bind _interactionactor (`self.InteractionActor`))
  (:`Pressed`
    (`/Engine/EditorBlueprintResources/StandardMacros.IsValid` _interactionactor
      (:`Is Valid`
        (set `/Game/01_Blueprint/BP_InteractionActor.IsInteracting` true _interactionactor))))
  (:`Released`
    (`/Engine/EditorBlueprintResources/StandardMacros.IsValid` _interactionactor
      (:`Is Valid`
        (set `/Game/01_Blueprint/BP_InteractionActor.IsInteracting` false _interactionactor)))))

(fn `UserConstructionScript`
  (`KismetArrayLibrary.Array_Add` (`SceneCaptureComponent.ShowOnlyActors` (`self.SceneCaptureComponent2D`)) self))