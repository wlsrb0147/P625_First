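; BP_DamageActor is a short-lived actor that displays a damage number through a widget component.
; Init_DamageActor takes a damage value and critical flag and forwards them to the WBP_DamageUI instance hosted by its Widget component.
; On BeginPlay it waits a fixed delay, then destroys itself, so each spawned instance cleans itself up.
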(event `self.ReceiveBeginPlay`
  (`KismetSystemLibrary.Delay` 2.0)
  (`self.K2_DestroyActor`))

(event `Init_DamageActor`
  (params (Damage :type Integer64) (Critical :type Boolean))
  (bind _aswbp_damage_ui (cast `/Game/01_Blueprint/03_Widget/WBP_DamageUI` (`WidgetComponent.GetWidget` (`self.Widget`))))
  (`/Game/01_Blueprint/03_Widget/WBP_DamageUI.Init_DamageUI` _aswbp_damage_ui Damage Critical))

(fn `UserConstructionScript`)