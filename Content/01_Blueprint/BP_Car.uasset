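; BP_Car is a pose-snapshot actor that shows a frozen copy of a skeletal mesh's pose with a dissolve effect.
; CopyPose copies the pose from a given skeletal component onto a PoseableMesh, then creates dynamic dissolve material instances across its material slots.
; Tick steadily lowers a DeltaTime variable at half real-time speed and feeds it into the "Dissolve (S)" parameter, with no clamp or actor cleanup.
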(event `self.ReceiveTick`
  (params (DeltaSeconds :type "Float (single-precision)"))
  (bind _output_get (set `self.DeltaTime` (- (`self.DeltaTime`) (/ DeltaSeconds 2.0))))
  (`MeshComponent.SetScalarParameterValueOnMaterials` (`self.PoseableMesh`) "Dissolve (S)" _output_get))

(event `CopyPose`
  (params (NewParam :type "SkeletalMeshComponent Object Reference"))
  (`PoseableMeshComponent.CopyPoseFromSkeletalComponent` (`self.PoseableMesh`) NewParam)
  (for _index (range 15)
    (`PrimitiveComponent.CreateDynamicMaterialInstance` (`self.PoseableMesh`) _index "/Game/01_Blueprint/02_Resource/Material/MTR_Deslove_Inst1.MTR_Deslove_Inst1" "None")))

(fn `UserConstructionScript`)